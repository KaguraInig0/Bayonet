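; BP_Stick is a world pickup for a melee stick that the third-person character can equip.
; A sphere overlap caches the character and enables input on the actor, and leaving the sphere disables it.
; While input is enabled, pressing E calls the character's EquipMelee with StickNiJustin and destroys the pickup.
; Each tick rotates the StickTxt label toward the player camera using a look-at rotation.
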(event `self.Sphere.OnComponentBeginOverlap`
  (params (OverlappedComponent :type "PrimitiveComponent Object Reference") (OtherActor :type "Actor Object Reference") (OtherComp :type "PrimitiveComponent Object Reference") (OtherBodyIndex :type Integer) (bFromSweep :type Boolean) (SweepResult :type "HitResult Structure (by ref)"))
  ;[1 1 1] When near the Stick
  (bind _asbp_third_person_character (cast `/Game/ThirdPerson/Blueprints/BP_ThirdPersonCharacter` OtherActor))
  (set `self.As BP Third Person Character` _asbp_third_person_character)
  (`self.EnableInput` (`GameplayStatics.GetPlayerController` 0)))

(event `self.Sphere.OnComponentEndOverlap`
  (params (OverlappedComponent :type "PrimitiveComponent Object Reference") (OtherActor :type "Actor Object Reference") (OtherComp :type "PrimitiveComponent Object Reference") (OtherBodyIndex :type Integer))
  ;[1 1 1] When near the Stick
  (cast `/Game/ThirdPerson/Blueprints/BP_ThirdPersonCharacter` OtherActor)
  (`self.DisableInput` (`GameplayStatics.GetPlayerController` 0)))

(event `self.ReceiveTick`
  (params (DeltaSeconds :type "Float (single-precision)"))
  ;[1 1 1] Text Rotation Relative to Character's Camera Location
  (`SceneComponent.K2_SetRelativeRotation` (`self.StickTxt`) (`KismetMathLibrary.FindLookAtRotation` (`self.K2_GetActorLocation`) (`self.K2_GetActorLocation` (`GameplayStatics.GetPlayerCameraManager` 0))) false false))

(event `Key|E`
  (params (Key :type "Key Structure"))
  (:`Pressed`
    (`/Game/ThirdPerson/Blueprints/BP_ThirdPersonCharacter.EquipMelee` (`self.As BP Third Person Character`) "/Game/Assets/Meshes/StickNiJustin.StickNiJustin")
    (`self.K2_DestroyActor`)))

(fn `UserConstructionScript`)